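; Player-controlled soldier pawn with world-axis movement, a hitscan automatic rifle, health and a kill counter; creates the player HUD on BeginPlay.
; Mouse velocity above a dead zone sets the target yaw, toward which control rotation interpolates each tick.
; Holding fire plays muzzle effects and looping audio while a timer repeats debug-drawn line traces from the muzzle socket, damaging hit actors.
; Incoming damage lowers health; death disables movement, aiming and fire input.
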(event EventTick
  (params (DeltaSeconds :type Float%20%28single-precision%29))
  (CallFunction|UpdatePlayerRotation))

(event EventBeginPlay
  (if (CallFunction|IsAlive)
    (bind _returnvalue (UserInterface|CreateWidget "/Game/UI/W_PlayerHUD.W_PlayerHUD_C" 0 self))
    (UserInterface|Viewport|AddtoViewport _returnvalue 0)))

(event Game|Damage|EventAnyDamage
  (params (Damage :type Float%20%28single-precision%29) (DamageType :type Damage%20Type%20Object%20Reference) (InstigatedBy :type Controller%20Object%20Reference) (DamageCauser :type Actor%20Object%20Reference))
  (bind _output_get (CallFunction|DecreaceHealth Damage))
  (if (<= _output_get 0.0)
    (Variables|Default|SetDead true)))

(event Input|ActionEvents|InputActionFireWeapon
  (params (Key :type Key%20Structure))
  (bind _returnvalue (CallFunction|IsAlive))
  (:Pressed
    (if _returnvalue
      (CallFunction|StartFiringWeapon)))
  (:Released
    (if _returnvalue
      (CallFunction|StopFiringWeapon))))

(event Input|AxisEvents|InputAxisMoveForeward
  (params (AxisValue :type Float%20%28single-precision%29))
  (if (CallFunction|IsAlive)
    (Pawn|Input|AddMovementInput "1.000000, 0, 0" AxisValue false)))

(event Input|AxisEvents|InputAxisMoveRightLeft
  (params (AxisValue :type Float%20%28single-precision%29))
  (if (CallFunction|IsAlive)
    (Pawn|Input|AddMovementInput "0,1.000000, 0" AxisValue false)))

(fn ConstructionScript)

(fn GetMouseVelocity
  (bind _returnvalue (Game|GetPlayerController 0))
  (bind (_deltax _deltay) (Class|PlayerController|GetInputMouseDelta _returnvalue))
  (return (/ (Math|Vector2D|MakeVector2D _deltax _deltay) (Utilities|Time|GetWorldDeltaSeconds))))

(fn UpdatePlayerRotation
  (bind _returnvalue (Game|GetPlayerController 0))
  (bind _returnvaluex (CallFunction|GetMouseVelocity))
  (bind (_x _y) (Math|Vector2D|BreakVector2D _returnvaluex))
  (if (and (CallFunction|IsMouseAboveDeltaZone) (CallFunction|IsAlive))
    (Pawn|SetControlRotation _returnvalue (Math|Interpolation|RInterpTo (Pawn|GetControlRotation _returnvalue :!class /Script/Engine.Controller) (Math|Rotator|MakeRotator 0.0 0.0 (Class|KismetMathLibrary|DegAtan2 _x _y)) (Utilities|Time|GetWorldDeltaSeconds) (Variables|Default|GetDeltaTimeMultiply)))))

(fn IsMouseAboveDeltaZone
  (return (> (Math|Vector2D|Vector2DLength (CallFunction|GetMouseVelocity)) (Variables|Default|GetDeadZone))))

(fn StartFiringWeapon
  (Components|Activation|Activate (Variables|Default|GetP_AssaultRifle_MF) false)
  (bind _returnvalue (Audio|SpawnSound2D "/Game/Sounds/Weapon_AssaultRifle/Stereo/SC_RandomFireloop.SC_RandomFireloop" 1.0 1.0 0.0 0))
  (Variables|Default|SetAudioFire1 _returnvalue)
  (CallFunction|WeaponTrace)
  (Utilities|Time|SetTimerbyFunctionName 0 "WeaponTrace" (Variables|Default|GetWeaponFireRate) true))

(fn StopFiringWeapon
  (bind _audiofire1 (Variables|Default|GetAudioFire1))
  (Utilities|IsValid _audiofire1
    (:Is%20Valid
      (Components|Activation|Deactivate (Variables|Default|GetP_AssaultRifle_MF))
      (Audio|Components|Audio|Stop _audiofire1)
      (Utilities|Time|ClearTimerbyFunctionName 0 "WeaponTrace")
      (if (CallFunction|IsAlive)
        (Audio|SpawnSound2D "/Game/Sounds/Weapon_AssaultRifle/Stereo/SC_„ShotEnd.SC_„ShotEnd" 1.0 1.0 0.0 0)))))

(fn DecreaceHealth
  (params (Input :type Float%20%28single-precision%29))
  (bind _output_get (Variables|Default|SetHealth (- (Variables|Default|GetHealth) Input)))
  (return _output_get))

(fn IsAlive
  (return (not (Variables|Default|GetDead))))

(fn WeaponTrace
  (bind _outhit (Collision|LineTraceByChannel (CallFunction|GetWeaponTraceStartLocation) (CallFunction|GetWeaponTraceEndLocation) "TraceTypeQuery1" false 0 "ForDuration"))
  (if (.bBlockingHit (Collision|BreakHitResult _outhit))
    (Game|Damage|ApplyDamage (.HitActor (Collision|BreakHitResult _outhit)) (Variables|Default|GetBaseDamage) 0 0)))

(fn GetWeaponTraceStartLocation
  (return (Transformation|GetSocketLocation (Variables|Default|GetRifle) "MuzzleFlashSocket")))

(fn GetWeaponTraceEndLocation
  (return (+ (CallFunction|GetWeaponTraceStartLocation) (* (Math|Vector|GetForwardVector (Pawn|GetControlRotation :!class /Script/Engine.Pawn)) (Variables|Default|GetWeaponRange)))))

(fn IncreaceKills
  (bind _result (Math|Integer|IncrementInt (Variables|Default|GetKills))
    (:%20%20
      (Variables|Default|SetKills _result))))