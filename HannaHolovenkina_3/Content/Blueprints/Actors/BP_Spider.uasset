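; BP_Spider is an enemy spider pawn that chases the player and plays an attack when close.
; On BeginPlay it moves toward the player with AIMoveTo, reissuing the move 0.2 seconds after each success.
; Each tick, if the player is within AttackRange and AM_Spider is not playing, it deactivates movement and plays a montage, restoring movement on completion.
; The file contains no damage logic.
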(event EventBeginPlay
  (AI|AIMoveTo self "0, 0, 0" (Game|GetPlayerCharacter 0) 5.0 false :!label _label
    (:OnSuccess
      (Utilities|FlowControl|Delay 0.2)
      (goto _label))))

(event Collision|EventActorBeginOverlap
  (params (OtherActor :type Actor%20Object%20Reference)))

(event EventTick
  (params (DeltaSeconds :type Float%20%28single-precision%29))
  (if (CallFunction|CanAttack)
    (Components|Activation|Deactivate (Variables|Character|GetCharacterMovement))
    (Animation|Montage|PlayMontage (Variables|Character|GetMesh) 0
      (:OnCompleted
        (Components|Activation|Activate (Variables|Character|GetCharacterMovement) false)))))

(fn ConstructionScript)

(fn CanAttack
  (return (and (CallFunction|IsAttackingRange) (not (CallFunction|IsAttacking)))))

(fn IsAttacking
  (return (Animation|Montage|MontageIsPlaying (Components|SkeletalMesh|GetAnimInstance (Variables|Character|GetMesh)) "/Game/Characters/Enemy_Great_Spider/Animations/AM_Spider.AM_Spider")))

(fn IsAttackingRange
  (return (< (Transformation|GetDistanceTo (Game|GetPlayerCharacter 0)) (Variables|Default|GetAttackRange))))